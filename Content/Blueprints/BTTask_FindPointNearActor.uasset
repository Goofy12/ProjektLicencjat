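; Behavior tree task that picks a random reachable navigation point near a target actor.
; It reads the actor from the ActorKey blackboard entry and searches within Radius of that actor's location.
; A found point is written to PointKey and the task succeeds; an invalid actor or failed search makes it fail.
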(event `self.ReceiveExecuteAI`
  (params (OwnerController :type "AIController Object Reference") (ControlledPawn :type "Pawn Object Reference"))
  (bind _returnvalue (`BTFunctionLibrary.GetBlackboardValueAsActor` (`self.ActorKey`)))
  (bind (_randomlocation _returnvalue_2) (`NavigationSystem.K2_GetRandomReachablePointInRadius` (`Actor.K2_GetActorLocation` _returnvalue) (`self.Radius`)))
  (`/Engine/EditorBlueprintResources/StandardMacros.IsValid` _returnvalue
    (:`Is Valid`
      (if _returnvalue_2
        (`BTFunctionLibrary.SetBlackboardValueAsVector` (`self.PointKey`) _randomlocation)
        (`self.FinishExecute` true)
        (else
          (`self.FinishExecute` false :!label _label))))
    (:`Is Not Valid`
      (goto _label))))