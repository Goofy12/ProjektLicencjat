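; Behavior tree service that lets an AI pawn detect the player as an enemy.
; On each tick it checks that player 0's character is valid, within SearchRadius and in the controller's line of sight.
; When all checks pass it writes the player to the EnemyKey blackboard entry, otherwise it clears that entry.
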(event `self.ReceiveTickAI`
  (params (OwnerController :type "AIController Object Reference") (ControlledPawn :type "Pawn Object Reference") (DeltaSeconds :type "Float (single-precision)"))
  (bind _returnvalue (`GameplayStatics.GetPlayerCharacter` 0))
  (`/Engine/EditorBlueprintResources/StandardMacros.IsValid` _returnvalue
    (:`Is Valid`
      (if (<= (`KismetMathLibrary.VSize` (- (`Actor.K2_GetActorLocation` ControlledPawn) (`Actor.K2_GetActorLocation` _returnvalue))) (`self.SearchRadius`))
        (if (`Controller.LineOfSightTo` OwnerController (`GameplayStatics.GetPlayerCharacter` 0) (0.0 0.0 0.0) false)
          (`BTFunctionLibrary.SetBlackboardValueAsObject` (`self.EnemyKey`) (`GameplayStatics.GetPlayerCharacter` 0))
          (else
            (`BTFunctionLibrary.SetBlackboardValueAsObject` (`self.EnemyKey`) :!label _label)))
        (else
          (goto _label))))
    (:`Is Not Valid`
      (goto _label))))