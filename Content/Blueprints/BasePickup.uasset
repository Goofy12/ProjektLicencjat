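; BasePickup is a base pickup actor that the first-person character collects by overlapping it.
; On overlap it checks CanPickup, which returns true by default, calls the empty OnPickup event, then disables collision and hides itself rather than being destroyed.
; OnActivator restores collision and visibility so the pickup can be collected again.
; A timeline for spinning the mesh's yaw exists but is never triggered.
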(event `self.ReceiveActorBeginOverlap`
  (params (OtherActor :type "Actor Object Reference"))
  (bind _asfirst_person_character (cast `/Game/FirstPersonBP/Blueprints/FirstPersonCharacter` OtherActor))
  (if (`self.CanPickup` _asfirst_person_character)
    (`self.OnPickup` _asfirst_person_character)
    (`self.SetActorEnableCollision` false)
    (`self.SetActorHiddenInGame` true)))

(event `OnPickup`
  (params (Player :type "/Game/FirstPersonBP/Blueprints/FirstPersonCharacter Object Reference")))

(event `/Game/Blueprints/ActivatorInterface.OnActivator`
  (`self.SetActorEnableCollision` true)
  (`self.SetActorHiddenInGame` false))

(fn `CanPickup`
  (params (player :type "/Game/FirstPersonBP/Blueprints/FirstPersonCharacter Object Reference"))
  (returns (canPickup :type Boolean))
  (return true))

(fn `UserConstructionScript`)