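; Behavior tree service that makes an AI-controlled TppCharacter shoot at the enemy stored in the blackboard.
; On each service tick it checks that the enemy is valid, in the controller's line of sight, within ShootDistance and inside ShootAngle of the pawn's forward vector, using a dot product against the cosine.
; When all checks pass, it fires a projectile along the pawn's own rotation rather than aiming at the enemy.
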(event `self.ReceiveTickAI`
  (params (OwnerController :type "AIController Object Reference") (ControlledPawn :type "Pawn Object Reference") (DeltaSeconds :type "Float (single-precision)"))
  (bind _returnvalue (`BTFunctionLibrary.GetBlackboardValueAsActor` (`self.EnemyKey`)))
  (bind _astpp_character (cast `/Game/Blueprints/TppCharacter` ControlledPawn))
  (`/Engine/EditorBlueprintResources/StandardMacros.IsValid` _returnvalue
    (:`Is Valid`
      (if (`Controller.LineOfSightTo` OwnerController _returnvalue (0.0 0.0 0.0) false)
        (bind _returnvalue_2 (- (`Actor.K2_GetActorLocation` _returnvalue) (`Actor.K2_GetActorLocation` _astpp_character)))
        (if (<= (`KismetMathLibrary.VSize` _returnvalue_2) (`self.ShootDistance`))
          (if (>= (`KismetMathLibrary.Dot_VectorVector` (`Actor.GetActorForwardVector` _astpp_character) (`KismetMathLibrary.Normal` _returnvalue_2)) (`KismetMathLibrary.DegCos` (`self.ShootAngle`)))
            (`/Game/Blueprints/TppCharacter.FireProjectile` _astpp_character (`Actor.K2_GetActorRotation` _astpp_character))))))))