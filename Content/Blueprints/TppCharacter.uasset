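; Third-person bot character that takes damage, shows a health bar when the player aims at it, and can fire projectiles.
; AnyDamage reduces Health; at zero it ragdolls the mesh, disables capsule collision, hides the widget and calls the Die dispatcher.
; Tick, throttled by a Delay, line-traces from the player's camera to toggle the health bar widget, which receives this bot as owner on BeginPlay.
; FireProjectile spawns a projectile and sound at the weapon's muzzle socket.
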(event `self.ReceiveAnyDamage`
  (params (Damage :type "Float (single-precision)") (DamageType :type "DamageType Object Reference") (InstigatedBy :type "Controller Object Reference") (DamageCauser :type "Actor Object Reference"))
  ;[1 1 1] zadawanie obrażeń
  (if (not (`self.isdeath`))
    (set `self.health` (`KismetMathLibrary.FMax` (- (`self.health`) Damage)))
    (if (`self.isdeath`)
      (`self.onDie`)
      (`self.EventDispatcherDie`))))

(event `onDie`
  (bind _mesh (`self.Mesh`))
  ;[1 1 1] smierc bota
  (`PrimitiveComponent.SetSimulatePhysics` _mesh true)
  (`PrimitiveComponent.SetCollisionProfileName` _mesh "Ragdoll")
  (`PrimitiveComponent.SetCollisionEnabled` _mesh "QueryAndPhysics")
  (`PrimitiveComponent.SetCollisionEnabled` (`self.CapsuleComponent`) "NoCollision")
  (`Widget.SetVisibility` (`WidgetComponent.GetUserWidgetObject` (`self.Widget`)) "Collapsed"))

(event `self.ReceiveTick`
  (params (DeltaSeconds :type "Float (single-precision)"))
  (bind _returnvalue (`GameplayStatics.GetPlayerCharacter` 0))
  ;[1 1 1] caly system trace i health bar
  (`KismetSystemLibrary.Delay` 0.1)
  (bind _asfirst_person_character (cast `/Game/FirstPersonBP/Blueprints/FirstPersonCharacter` _returnvalue))
  (bind _firstpersoncamera (`/Game/FirstPersonBP/Blueprints/FirstPersonCharacter.FirstPersonCamera` _asfirst_person_character))
  (bind _returnvalue_2 (`SceneComponent.K2_GetComponentLocation` _firstpersoncamera))
  (bind (_outhit _returnvalue_3) (`KismetSystemLibrary.LineTraceSingleByProfile` _returnvalue_2 (+ _returnvalue_2 (* (`SceneComponent.GetForwardVector` _firstpersoncamera) 3000.0)) "Pawn" true (`|MakeArray` _returnvalue :!type "Actor Object Reference") "None" false))
  (if (and _returnvalue_3 (== (`.HitActor` (`GameplayStatics.BreakHitResult` _outhit)) self))
    (`self.showHealthbar`)
    (else
      (`self.HideHealtBar`))))

(event `self.ReceiveBeginPlay`
  ;[1 1 1] caly system trace i health bar
  (bind _astpp_bothealth_bar_widget (cast `/Game/FirstPersonBP/Blueprints/TppBothealthBarWidget` (`WidgetComponent.GetUserWidgetObject` (`self.Widget`))))
  (set `/Game/FirstPersonBP/Blueprints/TppBothealthBarWidget.botowner` self _astpp_bothealth_bar_widget))

(event `HideHealtBar`
  ;[1 1 1] caly system trace i health bar
  (`Widget.SetVisibility` (`WidgetComponent.GetUserWidgetObject` (`self.Widget`)) "Collapsed"))

(event `showHealthbar`
  ;[1 1 1] caly system trace i health bar
  (`Widget.SetVisibility` (`WidgetComponent.GetUserWidgetObject` (`self.Widget`)) "Visible"))

(fn `FireProjectile`
  (params (FireRotation :type "Rotator Structure"))
  (bind _returnvalue (`SceneComponent.GetSocketLocation` (`self.WeaponMesh`) "Muzzle"))
  (`|SpawnActorFromClass` "/Game/FirstPersonBP/Blueprints/FirstPersonProjectile.FirstPersonProjectile_C" (`KismetMathLibrary.MakeTransform` _returnvalue FireRotation) "Undefined" "OverrideRootScale" null null)
  (`GameplayStatics.SpawnSoundAtLocation` "/Game/FirstPerson/Audio/FirstPersonTemplateWeaponFire02.FirstPersonTemplateWeaponFire02" _returnvalue (struct) 1.0 1.0 0.0 null null))

(fn `Getmaxhealth`
  (returns (maxhealth :type "Float (double-precision)"))
  (return (defaults `/Game/Blueprints/TppCharacter` (`GameplayStatics.GetObjectClass` self))))

(fn `isdeath`
  (returns (bisdeath :type Boolean))
  (return (<= (`self.health`) 0.0)))

(fn `UserConstructionScript`)